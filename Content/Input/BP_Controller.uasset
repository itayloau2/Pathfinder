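; Input controller for click-to-select, click-to-move control of BP_Character units, with a live path preview.
; It selects a BP_Character found at start; left-click traces pawns under the cursor to switch selection.
; Right-click sends the selected unit to the cursor hit using simple AI movement.
; Each tick, a synchronous navigation path to the cursor rebuilds a spline, drawn as short, raised debug-line segments.
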(event EventBeginPlay
  (bind _returnvalue (Actor|GetActorOfClass "/Game/Character/BP_Character.BP_Character_C"))
  (bind _output_get (Variables|Default|SetCurrentUnit _returnvalue))
  (Default|ToggleSelection _output_get true))

(event EventTick
  (params (DeltaSeconds :type Float%20%28single-precision%29))
  (bind _spline (Variables|Default|GetSpline))
  (bind _currentunit (Variables|Default|GetCurrentUnit))
  (Utilities|IsValid _currentunit
    (:Is%20Valid
      (bind _returnvalue (Class|NavigationSystemV1|FindPathtoLocationSynchronously (Transformation|GetActorLocation _currentunit) (.Location (Collision|BreakHitResult (.HitResult (Game|Player|GetHitResultUnderCursorbyChannel "TraceTypeQuery3" true)))) 0 0))
      (Spline|ClearSplinePoints (Variables|Default|GetSpline) true)
      (for _array_element (Variables|/Script/NavigationSystem.NavigationPath|GetPathPoints _returnvalue)
        (Spline|AddSplinePoint (Variables|Default|GetSpline) _array_element "World" true))
      (for _index (range 0 (Math|Float|Truncate (/ (Spline|GetSplineLength (Variables|Default|GetSpline)) 2e+01)))
        (Rendering|Debug|DrawDebugLine (+ (Spline|GetLocationatDistanceAlongSpline _spline (Math|Conversions|ToFloat(Integer) (* _index 20)) "World") "0.000000,0.000000,20.000000") (+ (Spline|GetLocationatDistanceAlongSpline _spline (Math|Conversions|ToFloat(Integer) (* (Math|Integer|Max(Integer) (- _index 1)) 20)) "World") "0.000000,0.000000,20.000000") "(R=0.000000,G=1.000000,B=0.000000,A=1.000000)" 0.0 5.0)))))

(event Input|MouseEvents|LeftMouseButton
  (params (Key :type Key%20Structure :default "None"))
  (:Pressed
    (bind _hitresult (Class|PlayerController|GetHitResultUnderCursorforObjects (Utilities|Array|MakeArray "ObjectTypeQuery3") true))
    (bind _asbp_character (Utilities|Casting|CastToBP_Character (.hitactor _hitresult)))
    (Utilities|IsValid 0
      (:Is%20Not%20Valid
        (if (== (Variables|Default|GetCurrentUnit) _asbp_character)
          (Default|ToggleSelection _asbp_character true)
          (Variables|Default|SetCurrentUnit _asbp_character)
          (else
            (Default|ToggleSelection (Variables|Default|GetCurrentUnit) false)
            (bind _output_get (Variables|Default|SetCurrentUnit _asbp_character))
            (Default|ToggleSelection _output_get true)))))))

(event Input|MouseEvents|RightMouseButton
  (params (Key :type Key%20Structure :default "None"))
  (bind _currentunit (Variables|Default|GetCurrentUnit))
  (:Pressed
    (Utilities|IsValid _currentunit
      (:Is%20Valid
        (bind _hitresult (Game|Player|GetHitResultUnderCursorbyChannel "TraceTypeQuery3" true))
        (AI|Navigation|SimpleMovetoLocation (Pawn|GetController _currentunit) (.Location (Collision|BreakHitResult _hitresult)))))))

(fn ConstructionScript)